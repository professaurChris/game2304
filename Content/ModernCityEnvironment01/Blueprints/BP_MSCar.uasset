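; BP_MSCar is a drivable car pawn with hold-to-open doors and configurable looks.
; Axis inputs and SpaceBar drive throttle, steering and handbrake; both look axes add pitch and yaw together to the spring arm.
; Q, E, R and F set door flags, which Tick interpolates into door angles on the AM_MSCar01 anim instance.
; The construction script applies light, exterior, window and interior materials plus spotlight intensity and colour.
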(event EventBeginPlay
  (bind _asam_mscar_01 (Utilities|Casting|CastToAM_MSCar01 (Components|SkeletalMesh|GetAnimInstance (Variables|Character|GetMesh))))
  (Variables|Default|SetAnim%20BP%20MSCar01 _asam_mscar_01))

(event EventTick
  (params (DeltaSeconds :type Float%20%28single-precision%29))
  (bind _returnvalue (Utilities|Time|GetWorldDeltaSeconds))
  (bind _anim_bp_mscar01 (Variables|Default|GetAnim%20BP%20MSCar01))
  (Variables|/Game/ModernCityEnvironment01/Blueprints/AM_MSCar01.AM_MSCar01_C|SetFLDoor _anim_bp_mscar01 (Math|Interpolation|FInterpTo (Variables|/Game/ModernCityEnvironment01/Blueprints/AM_MSCar01.AM_MSCar01_C|GetFLDoor _anim_bp_mscar01) (Math|Float|SelectFloat 6e+01 0.0 (Variables|Default|GetFLDoorOpen)) _returnvalue 3.0))
  (Variables|/Game/ModernCityEnvironment01/Blueprints/AM_MSCar01.AM_MSCar01_C|SetFRDoor _anim_bp_mscar01 (Math|Interpolation|FInterpTo (Variables|/Game/ModernCityEnvironment01/Blueprints/AM_MSCar01.AM_MSCar01_C|GetFRDoor _anim_bp_mscar01) (Math|Float|SelectFloat -6e+01 0.0 (Variables|Default|GetFRDoorOpen)) _returnvalue 3.0))
  (Variables|/Game/ModernCityEnvironment01/Blueprints/AM_MSCar01.AM_MSCar01_C|SetRRDoor _anim_bp_mscar01 (Math|Interpolation|FInterpTo (Variables|/Game/ModernCityEnvironment01/Blueprints/AM_MSCar01.AM_MSCar01_C|GetRRDoor _anim_bp_mscar01) (Math|Float|SelectFloat -6e+01 0.0 (Variables|Default|GetRRDoorOpen)) _returnvalue 3.0))
  (Variables|/Game/ModernCityEnvironment01/Blueprints/AM_MSCar01.AM_MSCar01_C|SetRLDoor _anim_bp_mscar01 (Math|Interpolation|FInterpTo (Variables|/Game/ModernCityEnvironment01/Blueprints/AM_MSCar01.AM_MSCar01_C|GetRLDoor _anim_bp_mscar01) (Math|Float|SelectFloat 6e+01 0.0 (Variables|Default|GetRLDoorOpen)) _returnvalue 3.0)))

(event Input|AxisEvents|InputAxisThrottle
  (params (AxisValue :type Float%20%28single-precision%29))
  (Class|WheeledVehicleMovementComponent|SetThrottleInput (Variables|Default|GetVehicleMovement) AxisValue))

(event Input|AxisEvents|InputAxisSteer
  (params (AxisValue :type Float%20%28single-precision%29))
  (Class|WheeledVehicleMovementComponent|SetSteeringInput (Variables|Default|GetVehicleMovement) AxisValue))

(event Input|AxisEvents|InputAxisLookRight
  (params (AxisValue :type Float%20%28single-precision%29))
  (Transformation|AddRelativeRotation (Variables|Default|GetSpringArm) (Math|Rotator|MakeRotator 0.0 (stale Input|AxisEvents|InputAxisLookUp AxisValue) AxisValue) false false))

(event Input|AxisEvents|InputAxisLookUp
  (params (AxisValue :type Float%20%28single-precision%29))
  (Transformation|AddRelativeRotation (Variables|Default|GetSpringArm) (Math|Rotator|MakeRotator 0.0 AxisValue (stale Input|AxisEvents|InputAxisLookRight AxisValue)) false false))

(event Input|KeyboardEvents|SpaceBar
  (params (Key :type Key%20Structure))
  (bind _vehiclemovement (Variables|Default|GetVehicleMovement))
  (:Pressed
    (Class|WheeledVehicleMovementComponent|SetHandbrakeInput _vehiclemovement true))
  (:Released
    (Class|WheeledVehicleMovementComponent|SetHandbrakeInput _vehiclemovement false)))

(event Input|KeyboardEvents|E
  (params (Key :type Key%20Structure))
  (:Pressed
    (Variables|Default|SetRLDoorOpen true))
  (:Released
    (Variables|Default|SetRLDoorOpen false)))

(event Input|KeyboardEvents|Q
  (params (Key :type Key%20Structure))
  (:Pressed
    (Variables|Default|SetRRDoorOpen true))
  (:Released
    (Variables|Default|SetRRDoorOpen false)))

(event Input|KeyboardEvents|F
  (params (Key :type Key%20Structure))
  (:Pressed
    (Variables|Default|SetFLDoorOpen true))
  (:Released
    (Variables|Default|SetFLDoorOpen false)))

(event Input|KeyboardEvents|R
  (params (Key :type Key%20Structure))
  (:Pressed
    (Variables|Default|SetFRDoorOpen true))
  (:Released
    (Variables|Default|SetFRDoorOpen false)))

(fn ConstructionScript
  (bind _mesh (Variables|Character|GetMesh))
  (bind _exterio_material (Variables|VehicleMaterial|GetExterio%20Material))
  (bind _window_material (Variables|VehicleMaterial|GetWindow%20Material))
  (bind _spotlight (Variables|Default|GetSpotLight))
  (bind _interior_material (Variables|VehicleMaterial|GetInterior%20Material))
  (bind _mesh_2 (Variables|Character|GetMesh))
  (bind _mesh_3 (Variables|Character|GetMesh))
  (Rendering|Material|SetMaterial (Variables|Character|GetMesh) 0 (Variables|VehicleMaterial|GetLight%20Material))
  (Rendering|Material|SetMaterial _mesh_2 1 _exterio_material)
  (Rendering|Material|SetMaterial _mesh_2 4 _exterio_material)
  (Rendering|Material|SetMaterial _mesh_2 7 _exterio_material)
  (Rendering|Material|SetMaterial _mesh_2 10 _exterio_material)
  (Rendering|Material|SetMaterial _mesh_2 14 _exterio_material)
  (Rendering|Material|SetMaterial _mesh_2 16 _exterio_material)
  (Rendering|Material|SetMaterial _mesh_3 3 _window_material)
  (Rendering|Material|SetMaterial _mesh_3 6 _window_material)
  (Rendering|Material|SetMaterial _mesh_3 9 _window_material)
  (Rendering|Material|SetMaterial _mesh_3 12 _window_material)
  (Rendering|Material|SetMaterial _mesh_3 15 _window_material)
  (Rendering|Material|SetMaterial _mesh 2 _interior_material)
  (Rendering|Material|SetMaterial _mesh 5 _interior_material)
  (Rendering|Material|SetMaterial _mesh 8 _interior_material)
  (Rendering|Material|SetMaterial _mesh 11 _interior_material)
  (Rendering|Material|SetMaterial _mesh 13 _interior_material)
  (Rendering|Components|Light|SetIntensity _spotlight (Variables|VehicleLight|GetLight%20Intensity))
  (Rendering|Components|Light|SetLightColor _spotlight (Variables|VehicleLight|GetLight%20Colour) true))