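; Drivable construction dump truck vehicle with a raising dumpster, back door and spring-arm camera.
; Input drives throttle, steering and handbrake, while both look axes share one spring-arm rotation node feeding pitch and yaw.
; Q and E set raise/open or lower/close targets, which Tick eases into AnimBP variables with FInterpTo.
; Construction Script applies materials and headlight settings; BeginPlay caches the AnimBP and runs a PhysX collision debug command.
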(event EventBeginPlay
  (Development|ExecuteConsoleCommand "PXVIS COLLISION")
  (bind _asab_ct01anim_blur_print (Utilities|Casting|CastToAB_CT01AnimBlurPrint (Components|SkeletalMesh|GetAnimInstance (Variables|Character|GetMesh))))
  (Variables|Default|SetCT01AnimBP _asab_ct01anim_blur_print))

(event EventTick
  (params (DeltaSeconds :type Float%20%28single-precision%29))
  (bind _returnvalue (Utilities|Time|GetWorldDeltaSeconds))
  (bind _ct01animbp (Variables|Default|GetCT01AnimBP))
  (Variables|/Game/ModernCityEnvironment01/Blueprints/AB_CT01AnimBlurPrint.AB_CT01AnimBlurPrint_C|SetDumpingGoingUpCT01 _ct01animbp (Math|Interpolation|FInterpTo (Variables|/Game/ModernCityEnvironment01/Blueprints/AB_CT01AnimBlurPrint.AB_CT01AnimBlurPrint_C|GetDumpingGoingUpCT01 _ct01animbp) (Math|Float|SelectFloat 2e+01 0.0 (Variables|Default|GetWantDumpsterGoUp)) _returnvalue 0.3))
  (Variables|/Game/ModernCityEnvironment01/Blueprints/AB_CT01AnimBlurPrint.AB_CT01AnimBlurPrint_C|SetBackDoorOpeningCT01 _ct01animbp (Math|Interpolation|FInterpTo (Variables|/Game/ModernCityEnvironment01/Blueprints/AB_CT01AnimBlurPrint.AB_CT01AnimBlurPrint_C|GetBackDoorOpeningCT01 _ct01animbp) (Math|Float|SelectFloat -6e+01 0.0 (Variables|Default|GetWantBackDoorOpen)) _returnvalue 0.3)))

(event Input|AxisEvents|InputAxisThrottle
  (params (AxisValue :type Float%20%28single-precision%29))
  (Class|WheeledVehicleMovementComponent|SetThrottleInput (Variables|Default|GetVehicleMovement) AxisValue))

(event Input|AxisEvents|InputAxisSteer
  (params (AxisValue :type Float%20%28single-precision%29))
  (Class|WheeledVehicleMovementComponent|SetSteeringInput (Variables|Default|GetVehicleMovement) AxisValue))

(event Input|AxisEvents|InputAxisLookRight
  (params (AxisValue :type Float%20%28single-precision%29))
  (Transformation|AddRelativeRotation (Variables|Default|GetSpringArm) (Math|Rotator|MakeRotator 0.0 (stale Input|AxisEvents|InputAxisLookUp AxisValue) AxisValue) false false))

(event Input|AxisEvents|InputAxisLookUp
  (params (AxisValue :type Float%20%28single-precision%29))
  (Transformation|AddRelativeRotation (Variables|Default|GetSpringArm) (Math|Rotator|MakeRotator 0.0 AxisValue (stale Input|AxisEvents|InputAxisLookRight AxisValue)) false false))

(event Input|KeyboardEvents|Q
  (params (Key :type Key%20Structure))
  (:Pressed
    (Variables|Default|SetWantDumpsterGoUp true)
    (Variables|Default|SetWantBackDoorOpen true)))

(event Input|KeyboardEvents|E
  (params (Key :type Key%20Structure))
  (:Pressed
    (Variables|Default|SetWantDumpsterGoUp false)
    (Variables|Default|SetWantBackDoorOpen false)))

(event Input|KeyboardEvents|SpaceBar
  (params (Key :type Key%20Structure))
  (bind _vehiclemovement (Variables|Default|GetVehicleMovement))
  (:Pressed
    (Class|WheeledVehicleMovementComponent|SetHandbrakeInput _vehiclemovement true))
  (:Released
    (Class|WheeledVehicleMovementComponent|SetHandbrakeInput _vehiclemovement false)))

(fn ConstructionScript
  (bind _mesh (Variables|Character|GetMesh))
  (bind _exterior_material (Variables|Material|GetExterior%20Material))
  (Rendering|Material|SetMaterial _mesh 0 _exterior_material)
  (Rendering|Material|SetMaterial _mesh 1 _exterior_material)
  (Rendering|Material|SetMaterial _mesh 2 (Variables|Material|GetLight%20Material))
  (Rendering|Material|SetMaterial _mesh 3 (Variables|Material|GetInterior%20Material))
  (Rendering|Material|SetMaterial _mesh 4 (Variables|Material|GetWheel%20Material))
  (Rendering|Material|SetMaterial _mesh 5 (Variables|Material|GetHydraulic%20Material))
  (Rendering|Components|Light|SetLightColor (Variables|Default|GetSpotLight1) (Variables|LightDetails|GetLight%20Colour) true)
  (Rendering|Components|Light|SetIntensity (Variables|Default|GetSpotLight) (Variables|LightDetails|GetLight%20Intensity)))